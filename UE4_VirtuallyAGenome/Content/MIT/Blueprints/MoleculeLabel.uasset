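; MoleculeLabel is a two-line text label actor that shows a molecule's tissue type and target gene.
; On BeginPlay it reads both fields from the "graph" object of ResponseObject and writes them to Textline0 and Textline1.
; Each line then shifts along relative Y by half its measured text Y size, offsetting it to suit the string it shows.
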(event `self.ReceiveBeginPlay`
  (bind _textline0 (`self.textline0`))
  (bind _textline1 (`self.textline1`))
  (bind _returnvalue (`VaRestJsonObject.GetObjectField` (`self.response object`) "graph"))
  (`TextRenderComponent.K2_SetText` _textline0 (`KismetTextLibrary.Conv_StringToText` (`VaRestJsonObject.GetStringField` _returnvalue "tissue_type")))
  (`SceneComponent.K2_SetRelativeLocation` _textline0 (`KismetMathLibrary.MakeVector` (.x (`SceneComponent.RelativeLocation` _textline0)) (+ (/ (.y (`TextRenderComponent.GetTextLocalSize` _textline0)) 2.0) (.y (`SceneComponent.RelativeLocation` _textline0))) (.z (`SceneComponent.RelativeLocation` _textline0))) false false)
  (`TextRenderComponent.K2_SetText` _textline1 (`KismetTextLibrary.Conv_StringToText` (`VaRestJsonObject.GetStringField` _returnvalue "target_gene")))
  (`SceneComponent.K2_SetRelativeLocation` _textline1 (`KismetMathLibrary.MakeVector` (.x (`SceneComponent.RelativeLocation` _textline1)) (+ (/ (.y (`TextRenderComponent.GetTextLocalSize` _textline1)) 2.0) (.y (`SceneComponent.RelativeLocation` _textline1))) (.z (`SceneComponent.RelativeLocation` _textline1))) false false))

(fn `UserConstructionScript`)