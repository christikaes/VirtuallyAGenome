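; MoleculeTarget actor that displays a 3D graph of genomic nodes (enhancer and CTCF peaks, SNPs and the like) fetched as JSON from a URL.
; On BeginPlay it requests the data, then spawns attached, scaled CPS actors typed and colored by color field; size-50 nodes get the Pax3 mesh without collision.
; A MoleculeLabel receives the JSON.
; Tick yaws the graph when rotation is enabled, pausing during Box overlap.
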(event `self.ReceiveBeginPlay`
  (bind _output_get (set `self.webrequest` (`VaRestRequestJSON.ConstructRequestExt` "GET" "x_www_form_urlencoded_url")))
  (add `VaRestRequestJSON.OnRequestComplete` _output_get (delegate `onComplete`))
  (`VaRestRequestJSON.ProcessURL` (`self.webrequest`) (`self.URL`)))

(event `onComplete`
  (params (Request :type "VaRestRequestJSON Object Reference"))
  (`KismetSystemLibrary.PrintString` (`KismetStringLibrary.Conv_ObjectToString` Request) false false)
  (bind _returnvalue (`VaRestRequestJSON.GetResponseObject` Request))
  (set `self.json` _returnvalue)
  (`KismetSystemLibrary.PrintString` "Directed Graph:")
  (`KismetSystemLibrary.PrintString` (`KismetStringLibrary.Conv_BoolToString` (`VaRestJsonObject.GetBoolField` _returnvalue "directed")) false)
  (bind _returnvalue_2 (`VaRestJsonObject.GetArrayField` _returnvalue "nodes"))
  (for _array_element _returnvalue_2
    (bind _returnvalue_3 (`VaRestJsonValue.AsObject` _array_element))
    (`KismetSystemLibrary.PrintString` (`VaRestJsonObject.GetStringField` _returnvalue_3 "name"))
    (bind _returnvalue_4 (`VaRestJsonObject.GetNumberField` _returnvalue_3 "size"))
    (bind _returnvalue_5 (`VaRestJsonObject.GetStringField` _returnvalue_3 "color"))
    (bind _returnvalue_6 (select `bool` (== _returnvalue_5 "purple") :`false` (select `bool` (== _returnvalue_5 "orange") :`false` (select `bool` (== _returnvalue_5 "grey") :`false` (select `bool` (== _returnvalue_5 "blue") :`false` (select `bool` (== _returnvalue_5 "green") :`false` (select `bool` (== _returnvalue_5 "red") :`true` 1) :`true` 2) :`true` 3) :`true` 4) :`true` 5) :`true` 6))
    (bind _returnvalue_7 (`|SpawnActorFromClass` "/Game/MIT/Blueprints/CPS.CPS_C" (`KismetMathLibrary.MakeTransform` (`KismetMathLibrary.MakeVector` (+ (.x (.location (`self.GetTransform` self))) (* (- (`KismetStringLibrary.Conv_StringToDouble` (`VaRestJsonObject.GetStringField` _returnvalue_3 "x")) 0.5) (`self.graphScale`))) (+ (.y (.location (`self.GetTransform` self))) (* (- (`KismetStringLibrary.Conv_StringToDouble` (`VaRestJsonObject.GetStringField` _returnvalue_3 "y")) 0.5) (`self.graphScale`))) (+ (.z (.location (`self.GetTransform` self))) (* (- (`KismetStringLibrary.Conv_StringToDouble` (`VaRestJsonObject.GetStringField` _returnvalue_3 "z")) 0.5) (`self.graphScale`)))) (.rotation (`self.GetTransform` self)) (`KismetMathLibrary.Conv_DoubleToVector` (* _returnvalue_4 (`self.size scale`)))) "AlwaysSpawn" "OverrideRootScale" null (`VaRestJsonObject.GetStringField` _returnvalue_3 "name") (`VaRestJsonObject.GetStringField` _returnvalue_3 "rsid") (`VaRestJsonObject.GetStringField` _returnvalue_3 "tfbs") (`VaRestJsonObject.GetStringField` _returnvalue_3 "cadd_score") (`VaRestJsonObject.GetStringField` _returnvalue_3 "deep_score") (`VaRestJsonObject.GetStringField` _returnvalue_3 "grasp_pheno ") (`VaRestJsonObject.GetStringField` _returnvalue_3 "gtex_eqtl_pval") (select `int` _returnvalue_6 :`0` "Unknown" :`1` "Enhancer Peak" :`2` "CTCF Peak" :`3` "SNCA Gene TSS" :`4` "Cohesion Peak" :`5` "SNP/CNV" :`6` "ATAC-Seq Peak")))
    (`self.K2_AttachToActor` _returnvalue_7 self "None" "KeepWorld" "KeepWorld" "KeepWorld" true)
    (if (`KismetMathLibrary.NearlyEqual_FloatFloat` _returnvalue_4 50.0)
      (bind _sphere (`/Game/MIT/Blueprints/CPS.Sphere` _returnvalue_7))
      (`StaticMeshComponent.SetStaticMesh` _sphere "/Game/MIT/models/pax3.pax3")
      (`PrimitiveComponent.SetMaterial` _sphere 0 "/Game/MIT/images/transparent.transparent")
      (bind _returnvalue_8 (select `int` _returnvalue_6 :`0` "/Game/Geometry/Meshes/CubeMaterial.CubeMaterial" :`1` "/Game/MIT/images/red256_Mat.red256_Mat" :`2` "/Game/MIT/images/green256_Mat.green256_Mat" :`3` "/Game/MIT/images/blue256_Mat.blue256_Mat" :`4` "/Game/MIT/images/grey256_Mat.grey256_Mat" :`5` "/Game/MIT/images/orange256_Mat.orange256_Mat" :`6` "/Game/MIT/images/purrple256_Mat.purrple256_Mat" :!type "MaterialInterface Object Reference"))
      (`PrimitiveComponent.SetMaterial` _sphere 1 _returnvalue_8)
      (`PrimitiveComponent.SetCollisionEnabled` _sphere "NoCollision")
      (else
        (`PrimitiveComponent.SetMaterial` _sphere 0 _returnvalue_8)))
    (`KismetArrayLibrary.Array_Add` (`self.ActorNodes`) _returnvalue_7))
  (`|SpawnActorFromClass` "/Game/MIT/Blueprints/MoleculeLabel.MoleculeLabel_C" (`KismetMathLibrary.MakeTransform` (- (.location (`SceneComponent.K2_GetComponentToWorld` (`self.label_anchor`))) (0.0 0.0 50.0)) (`KismetMathLibrary.MakeRotator` (.roll (.rotation (`SceneComponent.K2_GetComponentToWorld` (`self.label_anchor`)))) (.pitch (.rotation (`SceneComponent.K2_GetComponentToWorld` (`self.label_anchor`)))) (+ (.yaw (.rotation (`SceneComponent.K2_GetComponentToWorld` (`self.label_anchor`)))) -180.0)) (.scale (`SceneComponent.K2_GetComponentToWorld` (`self.label_anchor`)))) "AlwaysSpawn" "OverrideRootScale" null (`self.json`)))

(event `self.ReceiveTick`
  (params (DeltaSeconds :type "Float (single-precision)"))
  (bind _defaultsceneroot (`self.DefaultSceneRoot`))
  (if (and (`self.CanEverRotate`) (`self.Rotating`))
    (`SceneComponent.K2_SetWorldTransform` _defaultsceneroot (`KismetMathLibrary.MakeTransform` (.location (`SceneComponent.K2_GetComponentToWorld` _defaultsceneroot)) (`KismetMathLibrary.MakeRotator` 0.0 0.0 (+ (.yaw (.rotation (`SceneComponent.K2_GetComponentToWorld` _defaultsceneroot))) 0.1)) (.scale (`SceneComponent.K2_GetComponentToWorld` _defaultsceneroot))) false false)))

(event `self.Box.OnComponentBeginOverlap`
  (params (OverlappedComponent :type "PrimitiveComponent Object Reference") (OtherActor :type "Actor Object Reference") (OtherComp :type "PrimitiveComponent Object Reference") (OtherBodyIndex :type Integer) (bFromSweep :type Boolean) (SweepResult :type "HitResult Structure (by ref)"))
  ;[1 1 1] Stop rotating when near player
  (set `self.Rotating` false))

(event `self.Box.OnComponentEndOverlap`
  (params (OverlappedComponent :type "PrimitiveComponent Object Reference") (OtherActor :type "Actor Object Reference") (OtherComp :type "PrimitiveComponent Object Reference") (OtherBodyIndex :type Integer))
  ;[1 1 1] Stop rotating when near player
  (set `self.Rotating` true))

(fn `UserConstructionScript`)