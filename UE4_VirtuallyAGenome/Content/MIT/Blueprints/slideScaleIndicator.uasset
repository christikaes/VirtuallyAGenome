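; Actor for a sliding scale indicator that displays a reading as one of nine fixed positions.
; Every Tick rounds ScaleReading and uses it to select one of the marker components named 0 through 8.
; The Indicator component snaps to that marker's relative location and rotation while keeping its own scale, with no interpolation.
; ScaleReading is only read here, never set.
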(event `self.ReceiveTick`
  (params (DeltaSeconds :type "Float (single-precision)"))
  (`SceneComponent.K2_SetRelativeTransform` (`self.Indicator`) (`KismetMathLibrary.MakeTransform` (.location (`SceneComponent.GetRelativeTransform` (select `int` (`KismetMathLibrary.Round` (`self.ScaleReading`)) :`0` (`self.0`) :`1` (`self.1`) :`2` (`self.2`) :`3` (`self.3`) :`4` (`self.4`) :`5` (`self.5`) :`6` (`self.6`) :`7` (`self.7`) :`8` (`self.8`)))) (.rotation (`SceneComponent.GetRelativeTransform` (select `int` (`KismetMathLibrary.Round` (`self.ScaleReading`)) :`0` (`self.0`) :`1` (`self.1`) :`2` (`self.2`) :`3` (`self.3`) :`4` (`self.4`) :`5` (`self.5`) :`6` (`self.6`) :`7` (`self.7`) :`8` (`self.8`)))) (`SceneComponent.RelativeScale3D` (`self.Indicator`))) false false))

(fn `UserConstructionScript`)