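; Actor that builds a 3D molecule graph from JSON fetched over HTTP, then automatically zooms into one node.
; On BeginPlay, if WorldEnabled, it requests the URL and spawns attached Level0Node actors at scaled positions with colored dynamic materials.
; After a delay, a randomly picked node is enlarged and hidden, and a Level1GraphTarget spawns there to load its subgraph.
; Tick optionally spins the root and lerps its scale and location toward the zoom.
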(event `self.ReceiveBeginPlay`
  (set `self.graphScale_old` (`self.graphScale`))
  (if (`self.World_Enabled`)
    (bind _output_get (set `self.webrequest` (`VaRestRequestJSON.ConstructRequestExt` "GET" "x_www_form_urlencoded_url")))
    (add `VaRestRequestJSON.OnRequestComplete` _output_get (delegate `onComplete`))
    (`VaRestRequestJSON.ProcessURL` (`self.webrequest`) (`self.URL`))))

(event `onComplete`
  (params (Request :type "VaRestRequestJSON Object Reference"))
  (bind _level0nodes (`self.Level0Nodes`))
  (`KismetSystemLibrary.PrintString` (`KismetStringLibrary.Conv_ObjectToString` Request) false false)
  (bind _returnvalue (`VaRestRequestJSON.GetResponseObject` Request))
  (set `self.json` _returnvalue)
  (`KismetSystemLibrary.PrintString` "Directed Graph:")
  (`KismetSystemLibrary.PrintString` (`KismetStringLibrary.Conv_BoolToString` (`VaRestJsonObject.GetBoolField` _returnvalue "directed")) false)
  (bind _returnvalue_2 (`VaRestJsonObject.GetArrayField` _returnvalue "nodes"))
  (bind _output_get (set `self.json_Nodes` _returnvalue_2))
  (for (_array_element _array_index) _output_get
    (if true
      (bind _returnvalue_3 (`VaRestJsonValue.AsObject` _array_element))
      (bind _returnvalue_4 (`VaRestJsonObject.GetStringField` _returnvalue_3 "name"))
      (`KismetSystemLibrary.PrintString` _returnvalue_4 false)
      (bind _returnvalue_5 (`|SpawnActorFromClass` "/Game/MIT/Blueprints/Level0Node.Level0Node_C" (`KismetMathLibrary.MakeTransform` (`KismetMathLibrary.MakeVector` (+ (.x (.location (`self.GetTransform` self))) (* (- (`KismetStringLibrary.Conv_StringToDouble` (`VaRestJsonObject.GetStringField` _returnvalue_3 "x")) 0.0) (`self.graphScale`))) (+ (.y (.location (`self.GetTransform` self))) (* (- (`KismetStringLibrary.Conv_StringToDouble` (`VaRestJsonObject.GetStringField` _returnvalue_3 "y")) 0.0) (`self.graphScale`))) (+ (.z (.location (`self.GetTransform` self))) (* (- (`KismetStringLibrary.Conv_StringToDouble` (`VaRestJsonObject.GetStringField` _returnvalue_3 "z")) 0.0) (`self.graphScale`)))) (.rotation (`self.GetTransform` self)) (`KismetMathLibrary.Conv_DoubleToVector` 1.0)) "AlwaysSpawn" "OverrideRootScale" null _returnvalue_4 (`VaRestJsonObject.GetStringField` _returnvalue_3 "json_name")))
      (`KismetArrayLibrary.Array_Add` (`self.Level0Nodes`) _returnvalue_5)
      (`self.K2_AttachToActor` _returnvalue_5 self "None" "KeepRelative" "KeepRelative" "KeepRelative" true)
      (bind _sphere (`/Game/MIT/Blueprints/Level0Node.Sphere` _returnvalue_5))
      (bind _returnvalue_6 (`PrimitiveComponent.CreateDynamicMaterialInstance` _sphere 0 "/Game/MIT/images/RGBMat.RGBMat"))
      (bind _returnvalue_7 (`KismetStringLibrary.ParseIntoArray` (`KismetStringLibrary.LeftChop` (`KismetStringLibrary.RightChop` (`VaRestJsonObject.GetStringField` _returnvalue_3 "color") 4) 1) ","))
      (`MaterialInstanceDynamic.SetVectorParameterValue` _returnvalue_6 "RGB" (`KismetMathLibrary.Conv_VectorToLinearColor` (/ (`KismetMathLibrary.MakeVector` (`KismetStringLibrary.Conv_StringToDouble` (`KismetArrayLibrary.Array_Get` _returnvalue_7)) (`KismetStringLibrary.Conv_StringToDouble` (`KismetArrayLibrary.Array_Get` _returnvalue_7 1)) (`KismetStringLibrary.Conv_StringToDouble` (`KismetArrayLibrary.Array_Get` _returnvalue_7 2))) 255.0)))
      (`PrimitiveComponent.SetMaterial` _sphere 0 _returnvalue_6)))
  (`KismetArrayLibrary.Array_Shuffle` _level0nodes)
  (for _array_element_2 _level0nodes
    (`KismetSystemLibrary.K2_SetTimerDelegate` (delegate `CustomEvent_0`) 3.0)
    (break)))

(event `self.ReceiveTick`
  (params (DeltaSeconds :type "Float (single-precision)"))
  (bind _defaultsceneroot (`self.DefaultSceneRoot`))
  (bind _x (.x (`SceneComponent.K2_GetComponentScale` (`self.DefaultSceneRoot`))))
  (bind _returnvalue (`KismetMathLibrary.Lerp` _x (`self.graphScaleZoomTo`) (`self.AnimationLerp`)))
  (if (`self.World_Enabled`)
    (`|ExecutionSequence`
      (:`then_0`
        (if (`self.Rotating`)
          (`SceneComponent.K2_SetWorldTransform` _defaultsceneroot (`KismetMathLibrary.MakeTransform` (.location (`SceneComponent.K2_GetComponentToWorld` _defaultsceneroot)) (`KismetMathLibrary.MakeRotator` 0.0 0.0 (+ (.yaw (.rotation (`SceneComponent.K2_GetComponentToWorld` _defaultsceneroot))) 0.1)) (.scale (`SceneComponent.K2_GetComponentToWorld` _defaultsceneroot))) false false)))
      (:`then_1`
        (if (`KismetMathLibrary.NearlyEqual_FloatFloat` (`self.graphScaleZoomTo`) 0.0 0.0001)
          (set `self.graphScaleZoomTo` _x)
          (elif (not (`KismetMathLibrary.NearlyEqual_FloatFloat` _x (`self.graphScaleZoomTo`) 0.1))
            (set `self.AnimationLerp` (+ (`self.AnimationLerp`) 0.01))
            (`SceneComponent.SetWorldScale3D` (`self.DefaultSceneRoot`) (`KismetMathLibrary.Conv_DoubleToVector` _returnvalue))
            (`SceneComponent.K2_SetWorldLocation` (`self.DefaultSceneRoot`) (`KismetMathLibrary.VLerp` (* (`self.NodeToFollowStartWorld`) _returnvalue) (.location (`SceneComponent.K2_GetComponentToWorld` (`self.DefaultSceneRoot`))) (`self.AnimationLerp`)) false false)))))))

(event `CustomEvent_0`
  (`self.Select Next Level Graph` (stale `onComplete` _array_element_2)))

(event `Select Next Level Graph`
  (params (Node :type "/Game/MIT/Blueprints/Level0Node Object Reference"))
  (bind _nodetofollow (`self.NodeToFollow`))
  (bind _url_base (`self.URL_base`))
  (bind _json_name (`/Game/MIT/Blueprints/Level0Node.json_name` _nodetofollow))
  (set `self.NodeToFollow` Node)
  (`self.SetActorScale3D` Node (`KismetMathLibrary.Conv_DoubleToVector` 4.0))
  (set `self.graphScaleZoomTo` (* (.x (`SceneComponent.K2_GetComponentScale` (`self.DefaultSceneRoot`))) 10.0))
  (set `self.NodeToFollowStartWorld` (- (.location (`SceneComponent.K2_GetComponentToWorld` (`self.DefaultSceneRoot`))) (.location (`SceneComponent.K2_GetComponentToWorld` (`/Game/MIT/Blueprints/Level0Node.DefaultSceneRoot` (`self.NodeToFollow`))))))
  (`|SpawnActorFromClass` "/Game/MIT/Blueprints/Level1GraphTarget.Level1GraphTarget_C" (`self.GetTransform` _nodetofollow) "Undefined" "OverrideRootScale" null (`KismetStringLibrary.JoinStringArray` (`|MakeArray` _url_base _json_name) "") _url_base)
  (`KismetSystemLibrary.PrintString` "Trying to load a Lvl1 Graph from:")
  (`KismetSystemLibrary.PrintString` _json_name)
  (`SceneComponent.SetVisibility` (`/Game/MIT/Blueprints/Level0Node.Sphere` _nodetofollow) false false))

(fn `UserConstructionScript`)