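; Level 1 graph target actor that builds a 3D genomic node graph from web JSON.
; When WorldEnabled, BeginPlay GETs the URL, then spawns an attached CPS actor per node at scaled offsets, carrying annotation fields and an RGB-string-driven dynamic material.
; Node type always resolves to "Unknown".
; SelectNextLevelGraph enlarges a node and stores zoom and offset values, but Tick is empty and the timed auto-select chain is disconnected.
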(event Custom|onComplete
  (params (Request :type Va%20Rest%20Request%20JSON%20Object%20Reference))
  (bind _self self)
  (bind _returnvalue (Transformation|GetActorTransform _self))
  (bind (_location _rotation) (Math|Transform|BreakTransform _returnvalue))
  (bind (_x _y _z) (Math|Vector|BreakVector _location))
  ;[1 1 1] Spawn Current Level Graph
  (if false
    (Development|PrintString (Utilities|String|ToString(Object) Request) false false))
  (bind _returnvalue_2 (Class|VaRestRequestJSON|GetResponseObject Request))
  (Variables|Default|Setjson _returnvalue_2)
  (bind _returnvalue_3 (Class|VaRestJsonObject|GetArrayField _returnvalue_2 "nodes"))
  (bind _output_get (Variables|Default|Setjson_Nodes _returnvalue_3))
  (for (_array_element _array_index) _output_get
    (if true
      (bind _returnvalue_4 (Class|VaRestJsonValue|AsObject _array_element))
      (bind _returnvalue_5 (Game|SpawnActorfromClass "/Game/MIT/Blueprints/CPS.CPS_C" (Math|Transform|MakeTransform (Math|Vector|MakeVector (+ _x (* (- (Math|Conversions|ToFloat(Integer) (Class|VaRestJsonObject|GetStringField _returnvalue_4 "x")) 0.0) (Variables|Default|GetgraphScale))) (+ _y (* (- (Math|Conversions|ToFloat(Integer) (Class|VaRestJsonObject|GetStringField _returnvalue_4 "y")) 0.0) (Variables|Default|GetgraphScale))) (+ _z (* (- (Math|Conversions|ToFloat(Integer) (Class|VaRestJsonObject|GetStringField _returnvalue_4 "z")) 0.0) (Variables|Default|GetgraphScale)))) _rotation (Math|Conversions|ToVector(Float) 1.0)) "AlwaysSpawn" 0 (Class|VaRestJsonObject|GetStringField _returnvalue_4 "name") (Class|VaRestJsonObject|GetStringField _returnvalue_4 "rsid") (Class|VaRestJsonObject|GetStringField _returnvalue_4 "tfbs") (Class|VaRestJsonObject|GetStringField _returnvalue_4 "cadd_score") (Class|VaRestJsonObject|GetStringField _returnvalue_4 "deep_score") (Class|VaRestJsonObject|GetStringField _returnvalue_4 "grasp_pheno ") (Class|VaRestJsonObject|GetStringField _returnvalue_4 "gtex_eqtl_pval") (Utilities|Select :Index 0 :Option%200 "Unknown" :Option%201 "Enhancer Peak" :Option%202 "CTCF Peak" :Option%203 "SNCA Gene TSS" :Option%204 "Cohesion Peak" :Option%205 "SNP/CNV" :Option%206 "ATAC-Seq Peak")))
      (Utilities|Array|Add (Variables|Default|GetLevel0Nodes) 0)
      (Transformation|AttachActorToActor _returnvalue_5 self "None" "KeepWorld" "KeepWorld" "KeepWorld" true)
      (bind _returnvalue_6 (Rendering|Material|CreateDynamicMaterialInstance (Variables|/Game/MIT/Blueprints/CPS.CPS_C|GetSphere _returnvalue_5) 0 "/Game/MIT/images/RGBMat.RGBMat" :!class /Script/Engine.PrimitiveComponent))
      (Rendering|Material|SetVectorParameterValue _returnvalue_6 "RGB" (Math|Conversions|ToLinearColor(Vector) (Math|Vector|SelectVector (/ (Math|Vector|MakeVector (Math|Conversions|ToFloat(Integer) (Utilities|Array|Get(acopy) (Utilities|String|ParseIntoArray (Utilities|String|LeftChop (Utilities|String|RightChop (Class|VaRestJsonObject|GetStringField _returnvalue_4 "color") 4) 1) ","))) (Math|Conversions|ToFloat(Integer) (Utilities|Array|Get(acopy) (Utilities|String|ParseIntoArray (Utilities|String|LeftChop (Utilities|String|RightChop (Class|VaRestJsonObject|GetStringField _returnvalue_4 "color") 4) 1) ",") 1)) (Math|Conversions|ToFloat(Integer) (Utilities|Array|Get(acopy) (Utilities|String|ParseIntoArray (Utilities|String|LeftChop (Utilities|String|RightChop (Class|VaRestJsonObject|GetStringField _returnvalue_4 "color") 4) 1) ",") 2))) 255.0) "128.000000,128.000000, 0" (Class|KismetStringLibrary|IsNumeric (Utilities|Array|Get(acopy) (Utilities|String|ParseIntoArray (Utilities|String|LeftChop (Utilities|String|RightChop (Class|VaRestJsonObject|GetStringField _returnvalue_4 "color") 4) 1) ",") 2)))) :!class /Script/Engine.MaterialInstanceDynamic)
      (Rendering|Material|SetMaterial (Variables|/Game/MIT/Blueprints/CPS.CPS_C|GetSphere _returnvalue_5) 0 _returnvalue_6)))
  (Utilities|Array|Shuffle (Variables|Default|GetLevel0Nodes)))

(event Custom|CustomEvent_0
  (CallFunction|SelectNextLevelGraph (stale _array_element)))

(event Custom|Select%20Next%20Level%20Graph
  (params (Node :type Level%200%20Node%20Object%20Reference))
  ;[1 1 1] Spawn next level graph
  (Variables|Default|SetNodeToFollow Node)
  (Transformation|SetActorScale3D Node (Math|Conversions|ToVector(Float) 4.0))
  (Development|PrintString (Utilities|GetDisplayName Node))
  (Variables|Default|SetgraphScaleZoomTo (* (.X (Math|Vector|BreakVector (Transformation|GetWorldScale (Variables|Default|GetDefaultSceneRoot)))) 1e+01))
  (Variables|Default|SetNodeToFollowStartWorld (- (.Location (Math|Transform|BreakTransform (Transformation|GetWorldTransform (Variables|Default|GetDefaultSceneRoot)))) (.Location (Math|Transform|BreakTransform (Transformation|GetWorldTransform (Variables|/Game/MIT/Blueprints/Level0Node.Level0Node_C|GetDefaultSceneRoot (Variables|Default|GetNodeToFollow))))))))

(event EventBeginPlay
  (Development|PrintString "I am a new Level 1 Graph Target!")
  (Variables|Default|SetgraphScale_old (Variables|Default|GetgraphScale))
  (if (Variables|Default|GetWorld_Enabled)
    (bind _output_get (Variables|Default|Setwebrequest (Class|VaRestRequestJSON|ConstructRequestExt "GET" "x_www_form_urlencoded_url")))
    (EventDispatchers|BindEventtoOnRequestComplete _output_get (delegate Custom|onComplete))
    (Class|VaRestRequestJSON|ProcessURL (Variables|Default|Getwebrequest) (Variables|Default|GetURL))))

(event Collision|EventActorBeginOverlap
  (params (OtherActor :type Actor%20Object%20Reference)))

(event EventTick
  (params (DeltaSeconds :type Float%20%28single-precision%29)))

(fn ConstructionScript)